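; BP_SplinePlatform is a moving platform that travels back and forth along its spline, carrying a coin.
; On BeginPlay it spawns a BP_Coin and attaches it to the CoinSpot component.
; Each Tick advances a distance by Speed and Direction, reversing Direction at either end of the spline.
; The mesh takes the spline's local position at that distance, and its rotation too unless Locked is set.
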(event `Spawn Coin On Platform`
  ; Spawn Coin On Platform
  ;
  ; Pour l'ajout d'une pièce sur la plateforme, suivant les déplacement de cette dernière.
  ;
  ; 1. Fait apparaitre un acteur de type "BP_Coin".
  ; 2. Attache cet acteur au composant "CoinSpot" de notre acteur BP_SplinePlatform
  (bind _returnvalue (`|SpawnActorFromClass` "/Game/Blueprints/BP_Coin.BP_Coin_C" (`KismetMathLibrary.MakeTransform` (0.0 0.0 0.0)) "AlwaysSpawn" "MultiplyWithRoot" null null))
  (`self.K2_AttachToComponent` _returnvalue (`self.CoinSpot`) "None" "SnapToTarget" "KeepRelative" "KeepWorld" true))

(event `self.ReceiveBeginPlay`
  (`self.Spawn Coin On Platform`))

(event `self.ReceiveTick`
  (params (DeltaSeconds :type "Float (single-precision)"))
  (bind _distance (`self.Distance`))
  (bind (_returnvalue_location _returnvalue_rotation) (`KismetMathLibrary.BreakTransform` (`SplineComponent.GetTransformAtDistanceAlongSpline` (`self.Spline`) (`self.Distance`) "Local" false)))
  (bind (_returnvalue_location_2 _returnvalue_rotation_2 _returnvalue_scale) (`KismetMathLibrary.BreakTransform` (`SceneComponent.GetRelativeTransform` (`self.Mesh`))))
  (`|ExecutionSequence`
    (:`then_0`
      ; Calcul de la distance sur le spline selon la vitesse et la direction.
      (set `self.Distance` (+ (* (`self.Speed`) DeltaSeconds (`self.Direction`)) (`self.Distance`)))
      ; Modification de la direction si la plateforme atteint l'une des extremité du spline.
      (if (<= _distance 0.0)
        (set `self.Direction` 1)
        (elif (>= _distance (`SplineComponent.GetSplineLength` (`self.Spline`)))
          (set `self.Direction` -1))))
    (:`then_1`
      ; Actualise la position de la plateforme le long du spline.
      (`SceneComponent.K2_SetRelativeTransform` (`self.Mesh`) (`KismetMathLibrary.MakeTransform` _returnvalue_location (select `bool` (`self.Locked`) :`false` _returnvalue_rotation :`true` _returnvalue_rotation_2) _returnvalue_scale) false false))))

(fn `UserConstructionScript`)