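; BP_Button is an interactable button that shows a press animation and relays the interaction to another object.
; OnInteract starts PressedAnim, then calls OnInteract on InteractionOnPress with the same player if that reference is valid.
; PressedAnim replays a Timeline from the start, using its ButtonHeight track to lerp the CylinderButton's Z scale between UpScaleZ and DownScaleZ, so the button squashes rather than moves.
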(event `Pressed Anim`
  (bind _cylinder_button (`self.Cylinder Button`))
  (bind (_relativescale3d_x _relativescale3d_y) (`KismetMathLibrary.BreakVector` (`SceneComponent.RelativeScale3D` _cylinder_button)))
  ; Animation du bouton s'enfonçant.
  (bind (_direction _button_height) (`Timeline|Timeline` :!via `PlayFromStart`)
    (:`Update`
      (`SceneComponent.SetRelativeScale3D` _cylinder_button (`KismetMathLibrary.MakeVector` _relativescale3d_x _relativescale3d_y (`KismetMathLibrary.Lerp` (`self.Up Scale Z`) (`self.Down Scale Z`) _button_height))))))

(event `/Game/Blueprints/Interactions/BPI_Interactable.On Interact`
  (params (`Interacting Player` :type "/Game/ThirdPerson/Blueprints/BP_ThirdPersonCharacter Object Reference"))
  (bind _interactiononpress (`self.InteractionOnPress`))
  (`self.Pressed Anim`)
  (`/Engine/EditorBlueprintResources/StandardMacros.IsValid` _interactiononpress
    (:`Is Valid`
      (`/Game/Blueprints/Interactions/BPI_Interactable.On Interact` _interactiononpress `Interacting Player`))))

(fn `UserConstructionScript`
  (`parent.UserConstructionScript`))