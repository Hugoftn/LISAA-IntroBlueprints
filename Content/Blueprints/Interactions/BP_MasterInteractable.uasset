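; BP_MasterInteractable is a base interactable actor that registers itself with the player character when the player enters its interaction range.
; Overlap begin and end on InteractSphere notify BP_ThirdPersonCharacter of entering and leaving range, gated by the PlayerCanInteract flag that IsInteractable also exposes.
; The construction script sizes the sphere from InteractionSphereRadius, and OnInteract only prints a message naming the player and the interactable.
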(event `self.InteractSphere.OnComponentBeginOverlap`
  (params (OverlappedComponent :type "PrimitiveComponent Object Reference") (OtherActor :type "Actor Object Reference") (OtherComp :type "PrimitiveComponent Object Reference") (OtherBodyIndex :type Integer) (bFromSweep :type Boolean) (SweepResult :type "HitResult Structure (by ref)"))
  (if (`self.PlayerCanInteract`)
    (bind _asbp_third_person_character (cast `/Game/ThirdPerson/Blueprints/BP_ThirdPersonCharacter` OtherActor))
    (`/Game/ThirdPerson/Blueprints/BP_ThirdPersonCharacter.New Interaction In Range` _asbp_third_person_character self)))

(event `self.InteractSphere.OnComponentEndOverlap`
  (params (OverlappedComponent :type "PrimitiveComponent Object Reference") (OtherActor :type "Actor Object Reference") (OtherComp :type "PrimitiveComponent Object Reference") (OtherBodyIndex :type Integer))
  (if (`self.PlayerCanInteract`)
    (bind _asbp_third_person_character (cast `/Game/ThirdPerson/Blueprints/BP_ThirdPersonCharacter` OtherActor))
    (`/Game/ThirdPerson/Blueprints/BP_ThirdPersonCharacter.Interaction Out Of Range` _asbp_third_person_character self)))

(event `/Game/Blueprints/Interactions/BPI_Interactable.On Interact`
  (params (`Interacting Player` :type "/Game/ThirdPerson/Blueprints/BP_ThirdPersonCharacter Object Reference"))
  (`KismetSystemLibrary.PrintText` (`|FormatText` "{actor} interacted with {interactable}" (`KismetSystemLibrary.GetDisplayName` `Interacting Player`) (`KismetSystemLibrary.GetDisplayName` self))))

(fn `Is Interactable`
  (returns (Return :type Boolean))
  (return (`self.PlayerCanInteract`)))

(fn `UserConstructionScript`
  (`SphereComponent.SetSphereRadius` (`self.InteractSphere`) (`self.Interaction Sphere Radius`) true))