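; BP_AutomaticDoor is a door that opens when the third-person character enters its trigger box and closes when the character leaves.
; Box overlap events flip a direction value between forward and backward.
; Every tick, that direction and a speed advance a distance clamped to the spline length, and the Cube mesh takes the spline's local location and rotation at that distance while keeping its own scale.
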(event `self.ReceiveTick`
  (params (DeltaSeconds :type "Float (single-precision)"))
  (bind _cube (`self.Cube`))
  (bind _output_get (set `self.Distance` (`KismetMathLibrary.FClamp` (+ (* DeltaSeconds (`self.Speed`) (`self.Direction`)) (`self.Distance`)) 0.0 (`SplineComponent.GetSplineLength` (`self.Spline`)))))
  (bind (_returnvalue_location _returnvalue_rotation) (`KismetMathLibrary.BreakTransform` (`SplineComponent.GetTransformAtDistanceAlongSpline` (`self.Spline`) _output_get "Local" false)))
  (`SceneComponent.K2_SetRelativeTransform` _cube (`KismetMathLibrary.MakeTransform` _returnvalue_location _returnvalue_rotation (`SceneComponent.RelativeScale3D` _cube)) false false))

(event `self.Box.OnComponentBeginOverlap`
  (params (OverlappedComponent :type "PrimitiveComponent Object Reference") (OtherActor :type "Actor Object Reference") (OtherComp :type "PrimitiveComponent Object Reference") (OtherBodyIndex :type Integer) (bFromSweep :type Boolean) (SweepResult :type "HitResult Structure (by ref)"))
  (cast `/Game/ThirdPerson/Blueprints/BP_ThirdPersonCharacter` OtherActor)
  (set `self.Direction` 1.0))

(event `self.Box.OnComponentEndOverlap`
  (params (OverlappedComponent :type "PrimitiveComponent Object Reference") (OtherActor :type "Actor Object Reference") (OtherComp :type "PrimitiveComponent Object Reference") (OtherBodyIndex :type Integer))
  (cast `/Game/ThirdPerson/Blueprints/BP_ThirdPersonCharacter` OtherActor)
  (set `self.Direction` -1.0))

(fn `UserConstructionScript`)